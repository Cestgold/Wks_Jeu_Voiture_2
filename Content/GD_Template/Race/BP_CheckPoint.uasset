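; Race checkpoint actor that updates vehicle respawn points and reports the player's progress to the finish line.
; On BeginPlay it registers itself with its referenced FinishLine.
; Any overlapping BP_CustomPlayerVehicule gets the checkpoint's transform as its respawn position.
; Only the first pass by player 0's pawn sets Passed and notifies the FinishLine; this blueprint never resets that flag.
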(event EventBeginPlay
  ;[1 1 1] Se référencer à la finish line
  (Default|AddCheckpointtoList (Variables|Default|GetFinishLine) self))

(event Collision|EventActorBeginOverlap
  (params (OtherActor :type Actor%20Object%20Reference))
  ;[0.276 0.276 0.276] Collision avec une voiture
  (bind _asbp_custom_player_vehicule (Utilities|Casting|CastToBP_CustomPlayerVehicule OtherActor))
  (Default|SetRespawnPosition _asbp_custom_player_vehicule (Transformation|GetActorTransform))
  ;;[1 1 1] Si c'est le joueur, on valide le chekpoint
  (if (== OtherActor (Game|Player|GetPlayerPawn 0))
    (if (not (Variables|Default|GetPassed))
      (Variables|Default|SetPassed true)
      (Default|PassCheckpoint (Variables|Default|GetFinishLine)))))

(fn ConstructionScript)