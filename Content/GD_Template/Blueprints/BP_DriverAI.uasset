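; BP_DriverAI is an AI-driven vehicle that builds on a parent Blueprint for its race start and base behaviour.
; Each Tick runs turn, throttle and brake steps, whose macros push steering, throttle and brake values into the vehicle movement component.
; Braking also toggles the brake lights; the input values are not computed here.
; Line-trace helpers for centre-of-mass height and ground contact exist but are not called in live logic.
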(event Custom|Turn_AI
  (Utilities|TurnM))

(event Custom|Throttle_AI
  (Utilities|ThrottleM))

(event Custom|Brake_AI
  (Utilities|BrakeM))

(event EventBeginPlay
  (|CallParentFunction))

(event Collision|EventActorBeginOverlap
  (params (OtherActor :type Actor%20Object%20Reference)))

(event EventTick
  (params (DeltaSeconds :type Float%20%28single-precision%29))
  (|CallParentFunction DeltaSeconds)
  ;[1 1 1] AiControl
  (CallFunction|TurnAI)
  (CallFunction|ThrottleAI)
  (CallFunction|BrakeAI))

(event EventRaceStart
  (|CallParentFunction))

(fn ConstructionScript
  (|CallParentFunction))

(fn MesureVehiculeCommHeight
  (bind _returnvalue (Transformation|GetActorLocation))
  (bind _outhit (Collision|LineTraceByChannel _returnvalue (* _returnvalue (* (Math|Vector|VectorUp) 1e+03)) "TraceTypeQuery1" false 0 "None"))
  (return (- (.Z (Math|Vector|BreakVector _returnvalue)) (.Z (Math|Vector|BreakVector (.Location (Collision|BreakHitResult _outhit)))))))

(fn IsVehiculeonGround
  (bind _returnvalue (Transformation|GetActorLocation))
  (bind _returnvalue_2 (Collision|LineTraceByChannel _returnvalue (+ _returnvalue (* (Transformation|GetActorUpVector) (Variables|Default|GetCOMHeight) -1.5)) "TraceTypeQuery1" false 0 "ForDuration" true "(R=1.000000,G=0.000000,B=0.000000,A=1.000000)" "(R=0.000000,G=1.000000,B=0.000000,A=1.000000)" 0.2))
  (return _returnvalue_2))